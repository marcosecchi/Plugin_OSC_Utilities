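; Spot light Blueprint whose intensity and outer cone angle are driven remotely by data from an OSC server.
; On BeginPlay it binds a handler to the server's data update event.
; The handler prints each received command and value on screen, then switches on the command name to apply the value to the spot light component.
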(event Custom|OnData
  (params (Command :type String) (Data :type Float%20%28single-precision%29))
  (bind _spotlightcomponent (Variables|Default|GetSpotLightComponent))
  (Development|PrintString (Utilities|String|Append "Received Command: " Command " - with data: " (Utilities|String|ToString(Float) Data)) true false "(R=0.000000,G=0.660000,B=1.000000,A=1.000000)" 2.0 "LightCommand")
  (switch string Command
    (:SetIntensity
      (Rendering|Components|Light|SetIntensity _spotlightcomponent Data))
    (:SetOuterAngle
      (Rendering|Lighting|SetOuterConeAngle _spotlightcomponent Data))))

(event EventBeginPlay
  (EventDispatchers|BindEventtoOnDataUpdate (Variables|Default|GetOSCServer) (EventDispatchers|CreateEvent :!event Custom|OnData)))

(fn ConstructionScript)